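; Player state for a bomb-dropping game, tracking score, lives, death, bomb capacity and range, and level progress.
; A looping timer refills bombs one at a time, pausing at the maximum and resuming when a bomb is used.
; Update events change the stats, while getter functions expose them and gate bomb drops on ammo and death.
; Level-clear and key counters each activate the first Door found on reaching five, passing current and next level names.
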(event `self.ReceiveBeginPlay`
  (set `self.BombCount` (`self.MaxBombCount`))
  (bind _returnvalue (`KismetSystemLibrary.K2_SetTimer` null "RefillBomb" (`self.RefillTimer`) true))
  (set `self.Refill_TimeHandle` _returnvalue))

(event `/Game/_BluePrint/Managers/Interfaces/PlayerInterface.UpdateScore`
  (params (IN :type Integer))
  (set `self.PlayerScore` (+ (`self.PlayerScore`) IN)))

(event `/Game/_BluePrint/Managers/Interfaces/PlayerInterface.UpdateCurrentBomb`
  (set `self.BombCount` (- (`self.BombCount`) 1))
  (`KismetSystemLibrary.K2_UnPauseTimerHandle` (`self.Refill_TimeHandle`)))

(event `UpdateBombRangeModifier_1_1`
  (set `self.BombRangeModifier` (+ (`self.BombRangeModifier`) 1.0)))

(event `/Game/_BluePrint/Managers/Interfaces/PlayerInterface.UpdateLivesUp`
  (params (IN :type Integer))
  (bind _output_get (set `self.PlayerLives` (+ (`self.PlayerLives`) IN)))
  (set `self.PlayerLives` _output_get))

(event `/Game/_BluePrint/Managers/Interfaces/PlayerInterface.UpdateMaxBombs`
  (params (IN :type Integer))
  (set `self.MaxBombCount` (+ (`self.MaxBombCount`) IN)))

(event `/Game/_BluePrint/Managers/Interfaces/PlayerInterface.UpdateLives`
  (params (IN :type Integer))
  (set `self.PlayerLives` (- (`self.PlayerLives`) IN)))

(event `/Game/_BluePrint/Managers/Interfaces/PlayerInterface.SetDeadState`
  (params (DEAD :type Boolean))
  (set `self.Dead` DEAD))

(event `/Game/_BluePrint/Managers/Interfaces/PlayerInterface.UpdateLevelCleared`
  (bind _currentlvpt (`self.CurrentLVPt`))
  (set `self.CurrentLVPt` (+ _currentlvpt 1.0))
  (if (== _currentlvpt 5.0)
    (bind _outactors (`GameplayStatics.GetAllActorsOfClass` "/Game/_BluePrint/Enviroment/Door.Door_C"))
    (`/Game/_BluePrint/Enviroment/Door.Multi_ToggleActive` (`|GetArrayItem` _outactors) (`self.CurrentLevelName`) (`self.NextLevelName`))))

(event `/Game/_BluePrint/Managers/Interfaces/PlayerInterface.UpdateKeyClear`
  (bind _keypts (`self.KeyPts`))
  (set `self.KeyPts` (+ _keypts 1.0))
  (if (== _keypts 5.0)
    (bind _outactors (`GameplayStatics.GetAllActorsOfClass` "/Game/_BluePrint/Enviroment/Door.Door_C"))
    (`/Game/_BluePrint/Enviroment/Door.Multi_ToggleActive` (`|GetArrayItem` _outactors) (`self.CurrentLevelName`) (`self.NextLevelName`))))

(fn `RefillBomb`
  (if (== (`self.BombCount`) (`self.MaxBombCount`))
    (`KismetSystemLibrary.K2_PauseTimerHandle` (`self.Refill_TimeHandle`))
    (else
      (set `self.BombCount` (+ (`self.BombCount`) 1)))))

(fn `ReturnBombCount`
  (returns (OUT :type Integer))
  (return (`self.BombCount`)))

(fn `ReturnCanDropBomb`
  (returns (CanDrop :type Boolean))
  (return (and (> (`self.BombCount`) 0) (not (`self.Dead`)))))

(fn `ReturnPlayerLives`
  (returns (Lives :type Integer))
  (return (`self.PlayerLives`)))

(fn `ReturnPlayerScore`
  (returns (IN :type Integer))
  (return (`self.PlayerScore`)))

(fn `SetBombCount`
  (returns (BombCount :type Integer))
  (bind _output_get (set `self.BombCount` (`self.MaxBombCount`)))
  (return _output_get))

(fn `SetPlayerInputs`
  (returns (CanDrop :type Boolean) (CanMove :type Boolean) (Moving :type Boolean))
  (return (`self.CanDropBomb`) (`self.CanMove`) (`self.Moving`)))

(fn `SetPlayerLives`
  (returns (OUT :type Integer))
  (bind _output_get (set `self.PlayerLives` 3))
  (return _output_get))

(fn `UpdateBombRangeModifier`)

(fn `UserConstructionScript`)